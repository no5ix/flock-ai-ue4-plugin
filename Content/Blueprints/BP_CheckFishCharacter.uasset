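; Free-flying VR-enabled player character for viewing fish, turning on the HMD at BeginPlay.
; Input axes move it by unswept world offsets along the camera's forward and right vectors and world Z, and drive controller look.
; Holding Attract disables spline tick on FishLeaders within DistanceToCharacter of the camera; release re-enables it on all.
; Other inputs step movement speed and toggle the camera's pawn control rotation.
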(event `self.ReceiveBeginPlay`
  (`HeadMountedDisplayFunctionLibrary.EnableHMD` true))

(event `InputAxis|MoveUp`
  (params (AxisValue :type "Float (single-precision)"))
  (`self.K2_AddActorWorldOffset` (`KismetMathLibrary.MakeVector` 0.0 0.0 (* (`self.Speed`) AxisValue))))

(event `InputAction|SpeedDown`
  (params (Key :type "Key Structure" :default "AnyKey"))
  (:`Pressed`
    (bind _output_get (set `self.Speed` (+ (stale _output_get) -1.0)))
    (`KismetSystemLibrary.PrintString` (`KismetStringLibrary.Conv_DoubleToString` _output_get))))

(event `InputAction|SpeedUp`
  (params (Key :type "Key Structure" :default "AnyKey"))
  (:`Pressed`
    (bind _output_get (set `self.Speed` (+ (stale _output_get) 1.0)))
    (`KismetSystemLibrary.PrintString` (`KismetStringLibrary.Conv_DoubleToString` _output_get))))

(event `InputAxis|LookRight`
  (params (AxisValue :type "Float (single-precision)"))
  (`self.AddControllerYawInput` (* AxisValue (`self.TurnSpeed`))))

(event `InputAxis|LookUp`
  (params (AxisValue :type "Float (single-precision)"))
  (`self.AddControllerPitchInput` (* AxisValue (`self.TurnSpeed`))))

(event `InputAxis|MoveForward`
  (params (AxisValue :type "Float (single-precision)"))
  (`self.K2_AddActorWorldOffset` (* (`SceneComponent.GetForwardVector` (`self.CameraCpp`)) (* (`self.Speed`) AxisValue))))

(event `InputAxis|MoveRight`
  (params (AxisValue :type "Float (single-precision)"))
  (`self.K2_AddActorWorldOffset` (* (`SceneComponent.GetRightVector` (`self.CameraCpp`)) (* (`self.Speed`) AxisValue))))

(event `InputAction|Attract`
  (params (Key :type "Key Structure" :default "AnyKey"))
  (:`Pressed`
    (bind _outactors (`GameplayStatics.GetAllActorsOfClass` "/Script/MyFish.FishLeader"))
    (for _array_element _outactors
      (if (< (`KismetMathLibrary.VSize` (- (`self.K2_GetActorLocation` _array_element) (`SceneComponent.K2_GetComponentLocation` (`self.CameraCpp`)))) (`self.DistanceToCharacter`))
        (set `FishLeader.EnableSplineTick` false _array_element))))
  (:`Released`
    (bind _outactors_2 (`GameplayStatics.GetAllActorsOfClass` "/Script/MyFish.FishLeader"))
    (for _array_element_2 _outactors_2
      (set `FishLeader.EnableSplineTick` true _array_element_2))))

(event `InputAction|TogglePawnRotationSwitch`
  (params (Key :type "Key Structure" :default "AnyKey"))
  (bind _busepawncontrolrotation (`CameraComponent.bUsePawnControlRotation` (`self.CameraCpp`)))
  ;[1 1 1] Add R key for toggle pawn rotation switch
  (:`Pressed`
    (if _busepawncontrolrotation
      _
      (else
        _))
    (set `CameraComponent.bUsePawnControlRotation` (not _busepawncontrolrotation) (`self.CameraCpp`))))

(fn `UserConstructionScript`)