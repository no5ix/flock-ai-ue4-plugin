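; Spline actor that spawns a fish leader at a chosen spline point and drives its movement.
; BeginPlay passes two timer intervals to the leader; Tick advances it along the spline at a per-frame random speed, orienting it to the spline.
; Distance resets on reaching the first point, skipping the first match, to loop the path.
; When the leader's spline tick is disabled, it steps toward the player's camera at a frame-rate-dependent speed.
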(event `self.ReceiveBeginPlay`
  ;[1 1 1] Comment
  (bind _returnvalue (`|SpawnActorFromClass` (`self.LeaderClass`) (`KismetMathLibrary.MakeTransform` (`SplineComponent.GetLocationAtSplinePoint` (`self.Spline`) (`self.InitPointIndex`) "World")) "Undefined" "OverrideRootScale"))
  (bind _output_get (set `self.BPFishLeaderInst` _returnvalue))
  (set `FishLeader.AddLeaderTimerInterval` (`self.AddLeaderTimerInterval`) _output_get)
  (set `FishLeader.RemoveLeaderLocationInterval` (`self.RemoveLeaderLocationInterval`) _output_get)
  (set `self.Distance` (`SplineComponent.GetDistanceAlongSplineAtSplinePoint` (`self.Spline`) (`self.InitPointIndex`))))

(event `self.ReceiveTick`
  (params (DeltaSeconds :type "Float (single-precision)"))
  ;[1 1 1] Comment
  (if (`FishLeader.EnableSplineTick` (`self.BPFishLeaderInst`))
    (if (== (`SplineComponent.GetLocationAtDistanceAlongSpline` (`self.Spline`) (`self.Distance`) "World") (`SplineComponent.GetLocationAtSplinePoint` (`self.Spline`) 0 "World"))
      (if (`self.IsfirstTime`)
        (set `self.IsfirstTime` false)
        (else
          (set `self.Distance` 0.0))))
    (bind _output_get (set `self.Distance` (+ (stale _output_get) (* (`KismetMathLibrary.RandomFloatInRange` (`self.MinFishLeaderSpeed`) (`self.MaxFishLeaderSpeed`)) (`GameplayStatics.GetWorldDeltaSeconds`)))))
    (`self.K2_SetActorLocation` (`self.BPFishLeaderInst`) (`SplineComponent.GetLocationAtDistanceAlongSpline` (`self.Spline`) (`self.Distance`) "World") false false)
    (`self.K2_SetActorRotation` (`self.BPFishLeaderInst`) (`SplineComponent.GetRotationAtDistanceAlongSpline` (`self.Spline`) (`self.Distance`) "Local") false)
    (else
      (bind _ascheck_fish_character (cast `CheckFishCharacter` (`GameplayStatics.GetPlayerPawn` 0)))
      (`self.K2_AddActorWorldOffset` (`self.BPFishLeaderInst`) (* (`KismetMathLibrary.Normal` (- (`SceneComponent.K2_GetComponentLocation` (`CheckFishCharacter.CameraCpp` _ascheck_fish_character)) (`self.K2_GetActorLocation` (`self.BPFishLeaderInst`)))) (`self.MoveToHandSpeed`)) false false))))

(fn `UserConstructionScript`)