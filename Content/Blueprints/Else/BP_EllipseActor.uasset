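; Actor that moves its Cube component along an elliptical path in relative space.
; Each tick adds a fixed step to an angle, so speed depends on frame rate, then sets X and Y from cosine and sine scaled by long and short radii.
; Tick also unhides the actor whenever its hidden flag is set.
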(event `self.ReceiveTick`
  (params (DeltaSeconds :type "Float (single-precision)"))
  (bind _output_get (set `self.Radians` (+ 0.1 (stale _output_get))))
  (`SceneComponent.K2_SetRelativeLocation` (`self.Cube`) (`KismetMathLibrary.MakeVector` (* (`KismetMathLibrary.Cos` (`self.Radians`)) (`self.LongRadius`)) (* (`KismetMathLibrary.Sin` (`self.Radians`)) (`self.ShortRadius`))) false false)
  (if (`self.bHidden`)
    (`self.SetActorHiddenInGame` false)))

(fn `UserConstructionScript`)