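; BP_EllipseActorSpawner spawns a series of BP_EllipseActor instances at its own transform.
; A looping two-second timer, started on BeginPlay, drives each spawn and prints a debug message.
; Each new actor is hidden in game and receives the spawner's LongRadius and ShortRadius after spawning.
; A running Count clears the timer once it reaches Num.
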(event `self.ReceiveBeginPlay`
  (bind _returnvalue (`KismetSystemLibrary.K2_SetTimerDelegate` (delegate `CustomEvent_0`) 2.0 true)))

(event `CustomEvent_0`
  (bind (_returnvalue_location _returnvalue_rotation _returnvalue_scale) (`KismetMathLibrary.BreakTransform` (`self.GetTransform`)))
  (`KismetSystemLibrary.PrintString` "Hello")
  (bind _returnvalue (`|SpawnActorFromClass` "/Game/Blueprints/Else/BP_EllipseActor.BP_EllipseActor_C" (`KismetMathLibrary.MakeTransform` _returnvalue_location _returnvalue_rotation _returnvalue_scale) "AlwaysSpawn" "OverrideRootScale"))
  (`self.SetActorHiddenInGame` _returnvalue true)
  (set `/Game/Blueprints/Else/BP_EllipseActor.LongRadius` (`self.LongRadius`) _returnvalue)
  (set `/Game/Blueprints/Else/BP_EllipseActor.ShortRadius` (`self.ShortRadius`) _returnvalue)
  (bind _output_get (set `self.count` (+ (stale _output_get) 1)))
  (if (>= (`self.count`) (`self.Num`))
    (`KismetSystemLibrary.K2_ClearAndInvalidateTimerHandle` (stale `self.ReceiveBeginPlay` _returnvalue))))

(fn `UserConstructionScript`)