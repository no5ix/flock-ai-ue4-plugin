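; BP_Spiral is an actor that moves a Cube in a spiral along its SplinePath.
; On BeginPlay it stores the Cube's relative location as an offset, then plays a timeline that sets the distance along the spline.
; Each update rotates the offset by a fixed, frame-rate-dependent step around the spline direction.
; The Cube takes local X from the spline and Y/Z from the offset, ignoring the spline's own Y/Z.
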(event `self.ReceiveBeginPlay`
  (bind _splinepath (`self.SplinePath`))
  (bind _output_get (set `self.InitVector` (`SceneComponent.RelativeLocation` (`self.Cube`))))
  (bind (_direction _newtrack_0) (`Timeline|Timeline_0`)
    (:`Update`
      (bind _returnvalue (* _newtrack_0 (`SplineComponent.GetSplineLength` _splinepath)))
      (bind _output_get_2 (set `self.InitVector` (`KismetMathLibrary.RotateAngleAxis` (`self.InitVector`) 10.0 (`SplineComponent.GetDirectionAtDistanceAlongSpline` _splinepath _returnvalue "Local"))))
      (`SceneComponent.K2_SetRelativeLocation` (`self.Cube`) (`KismetMathLibrary.MakeVector` (.x (`SplineComponent.GetLocationAtDistanceAlongSpline` (`self.SplinePath`) _returnvalue "Local")) (.y _output_get_2) (.z _output_get_2)) false false))))

(fn `UserConstructionScript`)